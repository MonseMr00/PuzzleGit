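; BP_TriggerBox is a placement slot for an item puzzle.
; An overlapping BP_Item is released from its grabbed state and moved to the collision component's location.
; If their first tags match, it sets the Puzzle flag selected by its ItemEnum and calls ValidateItem.
; Any actor ending overlap clears that flag, without a type or tag check.
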(event EventBeginPlay)

(event Collision|EventActorBeginOverlap
  (params (OtherActor :type Actor%20Object%20Reference))
  (bind _puzzle (Variables|Default|GetPuzzle))
  (bind _asbp_item (Utilities|Casting|CastToBP_Item OtherActor))
  (Variables|/Game/LowPolyMedievalConstructions/Framework/CosasAle/BP_Item.BP_Item_C|SetIsGrabbed _asbp_item false)
  (Transformation|SetActorLocation OtherActor (Transformation|GetWorldLocation (Variables|Default|GetCollisionComponent)) false false)
  (if (== (Utilities|Array|Get(acopy) (Variables|Actor|GetTags)) (Utilities|Array|Get(acopy) (Variables|/Script/Engine.Actor|GetTags OtherActor)))
    (switch Utilities|FlowControl|Switch|SwitchonBP_ItemEnum (Variables|Default|GetItemEnum)
      (:NewEnumerator0
        (Variables|/Game/LowPolyMedievalConstructions/Framework/CosasAle/BP_Puzzle.BP_Puzzle_C|SetItem1 _puzzle true))
      (:NewEnumerator1
        (Variables|/Game/LowPolyMedievalConstructions/Framework/CosasAle/BP_Puzzle.BP_Puzzle_C|SetItem2 _puzzle true)))
    (Default|ValidateItem _puzzle)))

(event EventTick
  (params (DeltaSeconds :type Float%20%28single-precision%29)))

(event Collision|EventActorEndOverlap
  (params (OtherActor :type Actor%20Object%20Reference))
  (bind _puzzle (Variables|Default|GetPuzzle))
  (switch Utilities|FlowControl|Switch|SwitchonBP_ItemEnum (Variables|Default|GetItemEnum)
    (:NewEnumerator0
      (Variables|/Game/LowPolyMedievalConstructions/Framework/CosasAle/BP_Puzzle.BP_Puzzle_C|SetItem1 _puzzle false))
    (:NewEnumerator1
      (Variables|/Game/LowPolyMedievalConstructions/Framework/CosasAle/BP_Puzzle.BP_Puzzle_C|SetItem2 _puzzle false))))

(fn ConstructionScript)