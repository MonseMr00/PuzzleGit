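; Door actor Blueprint meant to swing its StaticMesh open when the O key is pressed.
; OpenDoor checks the Open flag and, while world yaw is at or above -90 degrees, lowers yaw at a speed scaled by DeltaTime.
; The key event calls it once with a zero DeltaTime, so the mesh does not turn.
; Tick is empty, and nothing in the graphs sets Open.
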(event EventBeginPlay)

(event Collision|EventActorBeginOverlap
  (params (OtherActor :type Actor%20Object%20Reference)))

(event EventTick
  (params (DeltaSeconds :type Float%20%28single-precision%29)))

(event Input|KeyboardEvents|O
  (params (Key :type Key%20Structure))
  (:Pressed
    (CallFunction|OpenDoor 0.0)))

(fn ConstructionScript)

(fn OpenDoor
  (params (DeltaTime :type Float%20%28double-precision%29))
  (bind _staticmesh (Variables|Default|GetStaticMesh))
  (bind _returnvalue (Transformation|GetWorldRotation _staticmesh))
  (if (Variables|Default|GetOpen)
    (if (<= (- -9e+01 (.yaw _returnvalue)) 0.0)
      (Transformation|SetWorldRotation _staticmesh (Math|Rotator|MakeRotator (.roll _returnvalue) (.pitch _returnvalue) (- (.yaw _returnvalue) (* DeltaTime 25.0))) false false))))